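; Runner obstacle Blueprint that kills the player character on overlap unless the character is sliding.
; On actor overlap it casts to BP_RUNNERCHARACTER and checks IsSliding.
; If not sliding, it calls the character's Death, then pauses the game after a short delay.
; BeginPlay and Tick are disabled, and the construction script only calls its parent.
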(event EventBeginPlay
  (|CallParentFunction) ; This node is disabled and will not be called.\nDrag off pins to build functionality.
)

(event EventTick
  (params (DeltaSeconds :type Float%20%28single-precision%29))
  (|CallParentFunction DeltaSeconds) ; This node is disabled and will not be called.\nDrag off pins to build functionality.
)

(event Collision|EventActorBeginOverlap
  (params (OtherActor :type Actor%20Object%20Reference))
  (bind _asbp_runnercharacter (Utilities|Casting|CastToBP_RUNNERCHARACTER OtherActor))
  (if (not (Variables|/Game/Runner/Blueprints/BP_RUNNERCHARACTER.BP_RUNNERCHARACTER_C|GetIs%20Sliding _asbp_runnercharacter))
    (Default|Death _asbp_runnercharacter)
    (Utilities|FlowControl|Delay 1.0)
    (Game|SetGamePaused true)))

(fn ConstructionScript
  (|CallParentFunction))